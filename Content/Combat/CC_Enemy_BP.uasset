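; CC_Enemy_BP is an AI enemy character Blueprint that exposes chase, stun and weapon controls.
; Chasing switches walk speed between jogging and a slower pace.
; DisableMovement runs on authority, applying a stun through the Blackboard, clearing AI focus and stopping movement, with a timer that only a longer duration can extend.
; Weapon toggling and attack combos are delegated to the Tools component and its active tool.
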(event `/Game/CharacterCustomizer/Combat/BPI_Combat.Chasing`
  (params (Chasing :type Boolean))
  (set `CharacterMovementComponent.MaxWalkSpeed` (select `bool` Chasing :`false` 150.0 :`true` (`self.Jog Speed`)) (`self.CharacterMovement`)))

(event `Toggle Stun`
  (params (BoolValue :type Boolean))
  (bind _returnvalue (`AIBlueprintHelperLibrary.GetAIController` self))
  (`BlackboardComponent.SetValueAsBool` (`self.Blackboard`) "Stunned" BoolValue)
  (if BoolValue
    (`AIController.K2_SetFocus` _returnvalue null)
    (`Controller.StopMovement` _returnvalue)))

(event `/Game/CharacterCustomizer/Character_Customizer/Data/BPI_CharacterCustomizer.Disable Movement`
  (params (Duration :type "Float (single-precision)"))
  (`/Engine/EditorBlueprintResources/ActorMacros.Switch Has Authority`
    (:`Authority`
      (if (> Duration (`KismetSystemLibrary.K2_GetTimerRemainingTimeHandle` (`self.Movement Timer`)))
        (bind _returnvalue (`KismetSystemLibrary.K2_SetTimerDelegate` (delegate `Disable Stun`) Duration))
        (set `self.Movement Timer` _returnvalue)
        (`self.Toggle Stun` true)))))

(event `Disable Stun`
  (`self.Toggle Stun` false)
  (`KismetSystemLibrary.K2_ClearAndInvalidateTimerHandle` (`self.Movement Timer`)))

(event `/Game/CharacterCustomizer/Combat/BPI_Combat.Toggle Weapon`
  (params (Attacking :type Boolean))
  (bind _tools (`self.Tools`))
  (if Attacking
    (`/Game/CharacterCustomizer/Tools/Data/Tools.Action 1` _tools)
    (else
      (`/Game/CharacterCustomizer/Tools/Data/Tools.Action Main` _tools))))

(fn `Attack Combo`
  (params (Count :type Integer))
  (bind _active_tool (`/Game/CharacterCustomizer/Tools/Data/Tools.Active Tool` (`self.Tools`))
    (:`then`
      (`/Game/CharacterCustomizer/Tools/A_Tool_Base.Attack Combo` _active_tool Count)
      (return))
    (:`else`)))

(fn `UserConstructionScript`
  (`parent.UserConstructionScript`))